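; BP_Character_Game is the playable character, handling Enhanced Input movement, look, jump and item pickup.
; On BeginPlay it adds its input mapping context through PC_Game; walking follows the control rotation.
; Interact runs a visibility line trace forward from the capsule, out to PickUpDistance, so it follows body facing rather than camera aim.
; A hit BP_Item is passed to the ACInventory component for pickup.
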(event `self.ReceiveBeginPlay`
  ;[1 1 1] Comment
  (bind _aspc_game (cast `/Game/_Mintbloom/Basics/PC_Game` (`GameplayStatics.GetPlayerController` 0)))
  (`EnhancedInputSubsystemInterface.AddMappingContext` (pcsubsystem `EnhancedInputLocalPlayerSubsystem` _aspc_game) "/Game/_Mintbloom/Basics/Input/IMP.IMP" 0 (struct)))

(event `EnhancedInput|/Game/_Mintbloom/Basics/Input/IA_Walk`
  (params (ActionValue :type "Vector2D Structure") (ElapsedSeconds :type "Float (double-precision)") (TriggeredSeconds :type "Float (double-precision)") (InputAction :type "InputAction Object Reference" :default "/Game/_Mintbloom/Basics/Input/IA_Walk.IA_Walk"))
  (bind (_x _y) (`KismetMathLibrary.BreakVector2D` ActionValue))
  (bind _returnvalue (`self.GetControlRotation`))
  (:`Triggered`
    ;[1 1 1] Comment
    (`self.AddMovementInput` (`KismetMathLibrary.GetRightVector` _returnvalue) _x)
    (`self.AddMovementInput` (`KismetMathLibrary.GetForwardVector` _returnvalue) _y)))

(event `EnhancedInput|/Game/_Mintbloom/Basics/Input/IA_Look`
  (params (ActionValue :type "Vector2D Structure") (ElapsedSeconds :type "Float (double-precision)") (TriggeredSeconds :type "Float (double-precision)") (InputAction :type "InputAction Object Reference" :default "/Game/_Mintbloom/Basics/Input/IA_Look.IA_Look"))
  (bind (_x _y) (`KismetMathLibrary.BreakVector2D` ActionValue))
  (:`Triggered`
    ;[1 1 1] Comment
    (`self.AddControllerYawInput` _x)
    (`self.AddControllerPitchInput` _y)))

(event `EnhancedInput|/Game/_Mintbloom/Basics/Input/IA_Jump`
  (params (ActionValue :type Boolean) (ElapsedSeconds :type "Float (double-precision)") (TriggeredSeconds :type "Float (double-precision)") (InputAction :type "InputAction Object Reference" :default "/Game/_Mintbloom/Basics/Input/IA_Jump.IA_Jump"))
  (:`Triggered`
    ;[1 1 1] Comment
    (`self.Jump`)))

(event `EnhancedInput|/Game/_Mintbloom/Basics/Input/IA_Interact`
  (params (ActionValue :type Boolean) (ElapsedSeconds :type "Float (double-precision)") (TriggeredSeconds :type "Float (double-precision)") (InputAction :type "InputAction Object Reference" :default "/Game/_Mintbloom/Basics/Input/IA_Interact.IA_Interact"))
  (bind _returnvalue (`SceneComponent.K2_GetComponentLocation` (`self.CapsuleComponent`)))
  (:`Triggered`
    (bind _outhit (`KismetSystemLibrary.LineTraceSingle` :`Start` _returnvalue :`End` (+ _returnvalue (* (`KismetMathLibrary.GetForwardVector` (`SceneComponent.K2_GetComponentRotation` (`self.CapsuleComponent`))) (`self.PickUp_Distance`))) :`TraceChannel` "TraceTypeQuery1" :`DrawTime` 1.0))
    (bind _asbp_item (cast `/Game/_Mintbloom/Items/_Common/BP_Item` (`.HitActor` (`GameplayStatics.BreakHitResult` _outhit))))
    (`/Game/_Mintbloom/Basics/AC_Inventory.F_Inventory_Item_PickUp` (`self.AC_Inventory`) _asbp_item)))

(fn `UserConstructionScript`)