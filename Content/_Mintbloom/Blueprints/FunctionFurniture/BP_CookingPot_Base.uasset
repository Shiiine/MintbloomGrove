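; BP_CookingPot_Base is the base Blueprint for a cooking pot, a piece of function furniture with its own inventory.
; On BeginPlay it sets its AttributeProvider to grade 1, then uses the truncated Capasity attribute as the ACInventory maximum size.
; GetItemType is an empty stub, and no cooking logic is defined in this Blueprint.
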(event `self.ReceiveBeginPlay`
  (`parent.ReceiveBeginPlay`)
  (`AttributeProviderComponent.SetCurrentGrade` (`self.AttributeProvider`) 1)
  (`/Game/_Mintbloom/Blueprints/Inventory/AC_Inventory.SetMaxInventorySize` (`self.AC_Inventory`) (`KismetMathLibrary.FTrunc` (`AttributeProviderComponent.GetAttributeValue` (`self.AttributeProvider`) (struct :`TagName` "Attribute.Capasity")))))

(fn `GetItemType`
  (returns (Type :type "GameplayTag Structure"))
  (return))

(fn `UserConstructionScript`
  (`parent.UserConstructionScript`))