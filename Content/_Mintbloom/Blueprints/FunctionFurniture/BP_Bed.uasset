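; Interactable bed that lets the player skip to a set day-cycle phase.
; On Interact it disables the pawn's input and has the game mode show a fade screen, then after a delay changes the day cycle and restores input.
; It then calls fast-forward, value-change and attribute-upgrade functions, which are still empty stubs, so resting currently has no effect on stats here.
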(event `/Game/_Mintbloom/Blueprints/Interface/WorldInteraction_I.Interact`
  (bind _returnvalue (`GameplayStatics.GetPlayerController` 0))
  (bind _returnvalue_2 (`GameplayStatics.GetPlayerController` 0))
  (`self.DisableInput` (`Controller.K2_GetPawn` _returnvalue_2) _returnvalue_2)
  (message `/Game/_Mintbloom/Blueprints/Interface/GM_Interaction_I.CreateFadeScreen` (`GameplayStatics.GetGameMode`) 6.0 2.0 2.0 (struct :`A` 1.0))
  (`KismetSystemLibrary.Delay` 4.0)
  (message `/Game/_Mintbloom/Blueprints/Interface/GM_Interaction_I.ChangeDayCycleTo` (`GameplayStatics.GetGameMode`) "NewEnumerator0")
  (`self.EnableInput` (`Controller.K2_GetPawn` _returnvalue) _returnvalue)
  (`self.FastForwardCalculation`)
  (`self.DecreaseIncreaseValue` 0.0)
  (`self.UpgradeAttribute`))

(fn `DecreaseIncreaseValue`
  (params (time :type "Float (double-precision)")))

(fn `FastForwardCalculation`
  (returns (SkipedTime :type "Float (double-precision)"))
  (return 0.0))

(fn `UpgradeAttribute`)

(fn `UserConstructionScript`
  (`parent.UserConstructionScript`))