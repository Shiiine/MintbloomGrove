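; BP_Meal is a meal item Blueprint that shows its food category as in-world text.
; Its construction script switches on the gameplay tag from GetItemBase and writes a short hard-coded label to a TextRender for each food type.
; GetItemBase and GetItemType only forward to the parent class, while Interact is an empty stub and the other events are disabled.
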(event `/Game/_Mintbloom/Blueprints/Interface/WorldInteraction_I.Interact`)

(fn `GetItemBase`
  (returns (ItemBase :type "GameplayTag Structure"))
  (bind _itembase (`parent.GetItemBase`))
  (return _itembase))

(fn `GetItemType`
  (returns (Type :type "GameplayTag Structure"))
  (bind _type (`parent.GetItemType`))
  (return _type))

(fn `UserConstructionScript`
  (`parent.UserConstructionScript`)
  (bind _itembase (`self.GetItemBase`))
  (`|SwitchGameplayTag` _itembase
    (:`Food.Type.BalancedFood`
      (`TextRenderComponent.K2_SetText` (`self.TextRender`) "Balance"))
    (:`Food.Type.Fatty`
      (`TextRenderComponent.K2_SetText` (`self.TextRender`) "Fatty"))
    (:`Food.Type.MeetFood`
      (`TextRenderComponent.K2_SetText` (`self.TextRender`) "Meet"))
    (:`Food.Type.Substantial`
      (`TextRenderComponent.K2_SetText` (`self.TextRender`) "Substan"))
    (:`Food.Type.UselesFood`
      (`TextRenderComponent.K2_SetText` (`self.TextRender`) "Useles"))
    (:`Food.Type.VeganFood`
      (`TextRenderComponent.K2_SetText` (`self.TextRender`) "Vegan"))))