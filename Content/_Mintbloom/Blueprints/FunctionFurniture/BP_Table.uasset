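; BP_Table is a table furniture actor that holds meals in four food sockets.
; The construction script fills a map from each socket component to an occupied flag, initially free.
; SpawnMeal spawns a BP_Meal at the first free socket, passing its slot index and meal type, then marks it occupied.
; IsTableEmpty returns a separate IsEmpty variable that these graphs never update, and nothing here frees a socket.
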(fn `IsTableEmpty`
  (returns (IsEmpty :type Boolean))
  (return (`self.IsEmpty`)))

(fn `SpawnMeal`
  (params (MealType :type "GameplayTag Structure"))
  (bind _food_socets (`self.Food Socets`))
  (bind _keys (`BlueprintMapLibrary.Map_Keys` _food_socets))
  (for (_array_element _array_index) _keys
    (if (== (`BlueprintMapLibrary.Map_Find` _food_socets _array_element) false)
      (`|SpawnActorFromClass` "/Game/_Mintbloom/Blueprints/FunctionFurniture/Food/BP_Meal.BP_Meal_C" (`KismetMathLibrary.MakeTransform` (`SceneComponent.K2_GetComponentLocation` _array_element)) "Undefined" "MultiplyWithRoot" null _array_index (struct) MealType null)
      (`BlueprintMapLibrary.Map_Add` (`self.Food Socets`) _array_element true)
      (return))))

(fn `UserConstructionScript`
  (`BlueprintMapLibrary.Map_Add` (`self.Food Socets`) (`self.FoodSocet2`))
  (`BlueprintMapLibrary.Map_Add` (`self.Food Socets`) (`self.FoodSocet3`))
  (`BlueprintMapLibrary.Map_Add` (`self.Food Socets`) (`self.FoodSocet4`))
  (`BlueprintMapLibrary.Map_Add` (`self.Food Socets`) (`self.FoodSocet1`)))