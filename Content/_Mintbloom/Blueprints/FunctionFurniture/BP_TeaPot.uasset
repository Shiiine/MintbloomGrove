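; Teapot furniture actor that the player interacts with as a crafting station.
; On BeginPlay it forces a fixed grade and sizes its inventory component from the capacity attribute.
; Interact, marked TBD, creates a WBP_TeaPot widget from the grade, inventory and result item, registers it on the player character, and anchors it left on the main HUD canvas.
; It exposes its inventory component, deferring item and grade accessors to the parent.
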(event `self.ReceiveBeginPlay`
  (`parent.ReceiveBeginPlay`)
  (`AttributeProviderComponent.SetCurrentGrade` (`self.AttributeProvider`) 3)
  (`/Game/_Mintbloom/Blueprints/Inventory/AC_Inventory.SetMaxInventorySize` (`self.AC_Inventory`) (`KismetMathLibrary.FTrunc` (`AttributeProviderComponent.GetAttributeValue` (`self.AttributeProvider`) (struct :`TagName` "Attribute.Capasity"))))
  (`self.SetGrade` 3))

(event `/Game/_Mintbloom/Blueprints/Interface/WorldInteraction_I.Interact`
  (bind _returnvalue (`GameplayStatics.GetPlayerController` 0))
  (bind _ac_inventory (`self.AC_Inventory`))
  ;[1 1 1] TBD
  (bind _items (message `/Game/_Mintbloom/Blueprints/Interface/InventoryInteraction_I.GetInventoryItems_i` _ac_inventory))
  (bind _grade (`self.GetGrade`))
  (bind _returnvalue_2 (`|CreateWidget` "/Game/_Mintbloom/Blueprints/UI/WBP_TeaPot.WBP_TeaPot_C" _returnvalue _grade _items (`/Game/_Mintbloom/Blueprints/Inventory/AC_Inventory.TeaPodResultItem` _ac_inventory) self))
  (bind _asbp_character_game (cast `/Game/_Mintbloom/Blueprints/BP_Character_Game` (`Controller.K2_GetPawn` _returnvalue)))
  (`/Game/_Mintbloom/Blueprints/BP_Character_Game.SetCurrentInteraction` _asbp_character_game (struct :`TagName` "ItemsType.CraftingStation") _returnvalue_2 self)
  (bind _hud (message `/Game/_Mintbloom/Blueprints/Interface/HUDInteraction_I.GetMainHUD` (`PlayerController.GetHUD` _returnvalue)))
  (bind _canvaspanel_21 (`/Game/_Mintbloom/Blueprints/UI/WBP_MainHUD.GetCanvasPanel` _hud))
  (bind _returnvalue_3 (`CanvasPanel.AddChildToCanvas` _canvaspanel_21 _returnvalue_2))
  (set `CanvasPanelSlot.bAutoSize` true _returnvalue_3)
  (`CanvasPanelSlot.SetAnchors` _returnvalue_3 (make `Anchors` (0.0 0.5) (0.0 0.5)))
  (`CanvasPanelSlot.SetPosition` _returnvalue_3 (100.0 -200.0)))

(fn `GetGrade`
  (returns (Grade :type Integer))
  (bind _grade (`parent.GetGrade`))
  (return _grade))

(fn `GetInventoryComponent`
  (returns (Component :type "ActorComponent Object Reference"))
  (return (`self.AC_Inventory`)))

(fn `GetItemBase`
  (returns (ItemBase :type "GameplayTag Structure"))
  (bind _itembase (`parent.GetItemBase`))
  (return _itembase))

(fn `GetItemType`
  (returns (Type :type "GameplayTag Structure"))
  (bind _type (`parent.GetItemType`))
  (return _type))

(fn `SetGrade`
  (params (Grade :type Integer))
  (returns (Grade_ :type Integer))
  (bind _grade_ (`parent.SetGrade` Grade))
  (return _grade_))

(fn `UserConstructionScript`
  (`parent.UserConstructionScript`))