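; Game mode for Mintbloom that hosts the asset manager and broadcasts day cycle changes.
; On BeginPlay it adds the MNG_Assets component from a class variable and binds a listener to the day cycle event.
; The Daycycle RepNotify fires that dispatcher with the new value, though the OnDayCycleChange_F handler is still empty.
; A getter exposes the manager's Items data assets.
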(event `self.ReceiveBeginPlay`
  (`|ExecutionSequence`
    (:`then_0`
      ;[1 1 1] Add MNG_Assets
      (bind _returnvalue (`|AddComponentByClass` (`self.Classs_MNG_Asseets`) self))
      (set `self.MNG_Asseets` _returnvalue))
    (:`then_1`
      (add `self.OnDayCycleChange` (`|CreateDelegate` :!event `OnDayCycleChange_F`)))))

(fn `GetAllItemsDataAsset`
  (returns (Items :type "Array of /Game/_Mintbloom/Blueprints/Inventory/STR_Item Structure"))
  (return (`/Game/_Mintbloom/Blueprints/AC_GameMode_MNG_Assets.Items` (`self.MNG_Asseets`))))

(fn `OnDayCycleChange_F`
  (params (NewDayCycle :type "/Game/_Mintbloom/Blueprints/Struct/DayCycle_E Enum" :default "NewEnumerator0")))

(fn `OnRep_Daycycle`
  (`self.OnDayCycleChange` (`self.Daycycle`)))

(fn `UserConstructionScript`)