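; BP_Item_Base is a base Blueprint for inventory items placed in the world.
; Its construction script sets the mesh and capsule collider from the STRItem struct, feeding ColliderHeight into radius and ColliderWidth into half-height.
; PickedUp destroys the actor, while FInteract is an empty event.
; GetItemNameID returns the struct's name as a string, and GetItemType defers to the parent implementation.
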(event `self.ReceiveBeginPlay`)

(event `/Game/_Mintbloom/Blueprints/Interface/ItemInteraction_I.F_Interact`)

(event `/Game/_Mintbloom/Blueprints/Interface/ItemInteraction_I.PickedUp`
  (`self.K2_DestroyActor`))

(fn `GetItemNameID`
  (returns (NameID :type String))
  (return (`KismetTextLibrary.Conv_TextToString` (`.Name_3_888C6473449A50127FEBC6B0306D6862` (break `/Game/_Mintbloom/Blueprints/Inventory/STR_Item` (`self.STR_Item`))))))

(fn `GetItemType`
  (returns (Type :type "GameplayTag Structure"))
  (bind _type (`parent.GetItemType`))
  (return _type))

(fn `UserConstructionScript`
  (bind (_nameid _name _description _icon _sm _collider_height _collider_width) (break `/Game/_Mintbloom/Blueprints/Inventory/STR_Item` (`self.STR_Item`)))
  (`StaticMeshComponent.SetStaticMesh` (`self.SM_Item`) _sm)
  (`CapsuleComponent.SetCapsuleSize` (`self.Collider`) _collider_height _collider_width true))