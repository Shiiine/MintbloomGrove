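; Player character with Enhanced Input movement, stamina, hunger and poison stats, and an inventory, all reflected on the main HUD.
; Construction loads gameplay-tagged attributes from a data table, and a looping timer updates the stats, with poison driving slowdown and a green screen-dirt effect.
; A camera line trace routes interactions by item-type tag to pickup, storage or generic interact; crafting is a stub.
; Consumables apply table-driven effects, and cheat-gated events override stats.
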(event `self.ReceiveTick`
  (params (DeltaSeconds :type "Float (single-precision)"))
  (`KismetSystemLibrary.PrintString` (`KismetStringLibrary.Conv_DoubleToString` (`KismetMathLibrary.VSize` (`MovementComponent.Velocity` (`self.CharacterMovement`)))) true true (struct :`G` 0.66 :`B` 1.0 :`A` 1.0) 0.0))

(event `self.ReceiveBeginPlay`
  (`|ExecutionSequence`
    (:`then_0`
      (bind _aspc_game (cast `/Game/_Mintbloom/Blueprints/PC_Game` (`GameplayStatics.GetPlayerController` 0)))
      (`EnhancedInputSubsystemInterface.AddMappingContext` (pcsubsystem `EnhancedInputLocalPlayerSubsystem` _aspc_game) "/Game/_Mintbloom/Blueprints/Input/IMP.IMP" 0 (struct)))
    (:`then_1`
      (`KismetSystemLibrary.K2_SetTimerDelegate` (`|CreateDelegate` :!event `RestorationTick`) 1.0 true)
      (bind _newparam (`/Game/_Mintbloom/Blueprints/UI/WBP_MainHUD.GetinventoryRef` (`self.GetUIHUD`)))
      (bind _conponent_ (`self.GetInventoryComponent`))
      (`/Game/_Mintbloom/Blueprints/UI/WBP_Inventory.InitializeInventory` _newparam (`/Game/_Mintbloom/Blueprints/Inventory/AC_Inventory.GetInventoryItems` _conponent_)))))

(event `HungerTick`
  (if (`self.ToggleHungerNeed`)
    (`self.SetCurrentHunger` (- (`self.GetCurrentHunger`) (`self.CurrentHungerRate`)))
    (`self.RefreshUIStatBar` (`self.GetCurrentHunger`) "NewEnumerator1")))

(event `RestorationTick`
  (if (not (`self.GetIsRunning`))
    (bind _output_get (`self.ChangeStaminaBy` (`self.CurrentStaminaRecovery`)))
    (`self.RefreshUIStatBar` _output_get))
  (`self.PoisonTick`)
  (`self.HungerTick`))

(event `PoisonTick`
  ;[1 1 1] ApplyAndRemovePoisonTick
  (if (`self.GetIsPoison`)
    (bind _return (`self.AddPoisoningBy` 1.0))
    (bind __ (`self.RefreshUIStatBar` _return "NewEnumerator2"))
    (`self.ApplyEffect` (struct :`TagName` "Effect.SlowMovementSpeed") (`KismetMathLibrary.FClamp` __ 0.0 0.3))
    (bind ((`PostProcessSettings` _postprocesssettings)) (make `PostProcessSettings` :`BloomDirtMask` "/Engine/MapTemplates/T_ScreenDirt02_w.T_ScreenDirt02_w" :`BloomDirtMaskIntensity` (* __ 2000.0) :`BloomDirtMaskTint` (struct :`R` 0.101122 :`G` 0.5 :`A` 1.0)))
    ;[1 1 1] Camera PP
    (set `CameraComponent.PostProcessSettings` _postprocesssettings (`self.GetCharacterCamera`))
    (else
      (bind _return_2 (`self.AddPoisoningBy` -1.0))
      (bind ___2 (`self.RefreshUIStatBar` _return_2 "NewEnumerator2"))
      (`self.ApplyEffect` (struct :`TagName` "Effect.SlowMovementSpeed") (`KismetMathLibrary.FClamp` ___2 0.0 0.3))
      (set `CameraComponent.PostProcessSettings` _postprocesssettings (`self.GetCharacterCamera`)))))

(event `EnhancedInput|/Game/_Mintbloom/Blueprints/Input/IA_Run`
  (params (ActionValue :type Boolean) (ElapsedSeconds :type "Float (double-precision)") (TriggeredSeconds :type "Float (double-precision)") (InputAction :type "InputAction Object Reference" :default "/Game/_Mintbloom/Blueprints/Input/IA_Run.IA_Run"))
  (:`Triggered`
    (if (> (`KismetMathLibrary.VSize` (`MovementComponent.Velocity` (`self.CharacterMovement`))) 0.01)
      (`KismetSystemLibrary.Delay` 0.5)
      (bind _output_get (`self.ChangeStaminaBy` -2.0))
      (`self.RefreshUIStatBar` _output_get)))
  (:`Started`
    (`self.SetIsRunning` true)
    (`self.SetCurrentWalkingSpeed` (* (`self.GetCurrentWalkingSpeed`) (`self.CurrentRunningSpeedMult`))))
  (:`Completed`
    (`self.SetIsRunning` false)
    (`self.SetCurrentWalkingSpeed` (`self.GetAttributeValueByTag` (struct :`TagName` "Attribute.MovementSpeed")))))

(event `EnhancedInput|/Game/_Mintbloom/Blueprints/Input/IA_Walk`
  (params (ActionValue :type "Vector2D Structure") (ElapsedSeconds :type "Float (double-precision)") (TriggeredSeconds :type "Float (double-precision)") (InputAction :type "InputAction Object Reference" :default "/Game/_Mintbloom/Blueprints/Input/IA_Walk.IA_Walk"))
  (bind (_x _y) (`KismetMathLibrary.BreakVector2D` ActionValue))
  (bind _returnvalue (`self.GetControlRotation`))
  (:`Triggered`
    (set `CharacterMovementComponent.MaxWalkSpeed` (* (`self.GetCurrentWalkingSpeed`) (- 1.0 (`self.GetSlowEffect`))) (`self.CharacterMovement`))
    ;[1 1 1] Comment
    (`self.AddMovementInput` (`KismetMathLibrary.GetRightVector` _returnvalue) _x)
    (`self.AddMovementInput` (`KismetMathLibrary.GetForwardVector` _returnvalue) _y)
    (bind _isinteract (`self.GetIsInteract`))
    (if _isinteract
      (`self.CloseCurrentInteraction`)
      (`self.CloseCurrentInteraction`))))

(event `EnhancedInput|/Game/_Mintbloom/Blueprints/Input/IA_Look`
  (params (ActionValue :type "Vector2D Structure") (ElapsedSeconds :type "Float (double-precision)") (TriggeredSeconds :type "Float (double-precision)") (InputAction :type "InputAction Object Reference" :default "/Game/_Mintbloom/Blueprints/Input/IA_Look.IA_Look"))
  (bind (_x _y) (`KismetMathLibrary.BreakVector2D` ActionValue))
  (:`Triggered`
    ;[1 1 1] Comment
    (bind _isinteract (`self.GetIsInteract`))
    (if (not _isinteract)
      (`self.AddControllerYawInput` _x)
      (`self.AddControllerPitchInput` _y))))

(event `EnhancedInput|/Game/_Mintbloom/Blueprints/Input/IA_Jump`
  (params (ActionValue :type Boolean) (ElapsedSeconds :type "Float (double-precision)") (TriggeredSeconds :type "Float (double-precision)") (InputAction :type "InputAction Object Reference" :default "/Game/_Mintbloom/Blueprints/Input/IA_Jump.IA_Jump"))
  (:`Started`
    ;[1 1 1] Comment
    (`self.Jump`)
    (if (`|EnumEquality` (`CharacterMovementComponent.MovementMode` (`self.CharacterMovement`)) "MOVE_Walking")
      (bind _output_get (`self.ChangeStaminaBy` -20.0))
      (`/Game/_Mintbloom/Blueprints/UI/WBP_MainHUD.SetStaminaBar` (`self.GetUIHUD`) (/ _output_get 100.0)))))

(event `EnhancedInput|/Game/_Mintbloom/Blueprints/Input/IA_Interact`
  (params (ActionValue :type Boolean) (ElapsedSeconds :type "Float (double-precision)") (TriggeredSeconds :type "Float (double-precision)") (InputAction :type "InputAction Object Reference" :default "/Game/_Mintbloom/Blueprints/Input/IA_Interact.IA_Interact"))
  (bind _returnvalue (`SceneComponent.K2_GetComponentLocation` (`self.GetCharacterCamera`)))
  (:`Started`
    (bind _isinteract (`self.GetIsInteract`))
    (if _isinteract
      (`self.CloseCurrentInteraction`)
      (`self.CloseCurrentInteraction`)
      (else
        (bind _outhit (`KismetSystemLibrary.LineTraceSingle` _returnvalue (+ _returnvalue (* (`SceneComponent.GetForwardVector` (`self.GetCharacterCamera`)) (`self.PickUp_Distance`))) "TraceTypeQuery1" false (`|MakeArray` self :!type "Actor Object Reference") (select `bool` (`MintbloomFunctionalLibrary.GetPlayInEditor`) :`true` "ForDuration" :!type "EDrawDebugTrace Enum") true (struct :`R` 1.0 :`A` 1.0) (struct :`G` 1.0 :`A` 1.0) 1.0))
        (bind (_bblockinghit _binitialoverlap _time _distance _location _impactpoint _normal _impactnormal _physmat _hitactor) (`GameplayStatics.BreakHitResult` _outhit))
        (`/Engine/EditorBlueprintResources/StandardMacros.IsValid` _hitactor
          (:`Is Valid`
            (`self.Interact` _hitactor)))))))

(event `EnhancedInput|/Game/_Mintbloom/Blueprints/Input/IA_Backpack`
  (params (ActionValue :type Boolean) (ElapsedSeconds :type "Float (double-precision)") (TriggeredSeconds :type "Float (double-precision)") (InputAction :type "InputAction Object Reference" :default "/Game/_Mintbloom/Blueprints/Input/IA_Backpack.IA_Backpack"))
  (:`Started`
    (bind _currently (`self.ShowHideInventory`))
    (`self.ShowHideMouseCursor` _currently)))

(event `/Game/_Mintbloom/Blueprints/Interface/PawnInteraction_I.ConsumeItem`
  (params (ItemID :type String))
  (bind (_effect _value) (`self.FindEffectByItemID` ItemID))
  (`self.ApplyEffect` _effect _value))

(event `EnableCheats`
  (params (NewParam :type Boolean))
  (set `self.CheatEnable` NewParam))

(event `SetStaminaRecovery`
  (params (NewParam :type "Float (double-precision)"))
  (if (`self.AllowCheat`)
    (set `self.CurrentStaminaRecovery` NewParam)))

(event `SetMaximumStamina`
  (params (NewParam :type "Float (double-precision)"))
  (if (`self.AllowCheat`)
    (set `self.CurrentMaximumStamina` NewParam)))

(event `GetPoisoned`
  (params (NewParam :type Boolean))
  (if (`self.AllowCheat`)
    (`self.SetIsPoison` NewParam)))

(event `AddPoisonBar`
  (params (NewParam :type "Float (double-precision)"))
  (if (`self.AllowCheat`)
    (bind _return (`self.AddPoisoningBy` NewParam))
    (bind __ (`self.RefreshUIStatBar` _return "NewEnumerator2"))
    (`self.ApplyEffect` (struct :`TagName` "Effect.SlowMovementSpeed") (`KismetMathLibrary.FClamp` __ 0.0 0.3))
    (set `CameraComponent.PostProcessSettings` (make `PostProcessSettings` :`BloomDirtMask` "/Engine/MapTemplates/T_ScreenDirt02_w.T_ScreenDirt02_w" :`BloomDirtMaskIntensity` (* __ 2000.0) :`BloomDirtMaskTint` (struct :`R` 0.101122 :`G` 0.5 :`A` 1.0)) (`self.GetCharacterCamera`))))

(event `SetHungerBar`
  (params (NewParam :type "Float (double-precision)"))
  (if (`self.AllowCheat`)
    (`self.SetCurrentHunger` NewParam)
    (`self.RefreshUIStatBar` (`self.GetCurrentHunger`) "NewEnumerator1")))

(event `TogleHungerNeed`
  (params (NewParam :type Boolean))
  (if (`self.AllowCheat`)
    (set `self.ToggleHungerNeed` NewParam)))

(event `SetHungerRate`
  (params (CurrentHungerRate :type "Float (double-precision)"))
  (if (`self.AllowCheat`)
    (set `self.CurrentHungerRate` CurrentHungerRate)))

(event `SetSpeed`
  (params (MS :type "Float (double-precision)"))
  (if (`self.AllowCheat`)
    (`self.SetCurrentWalkingSpeed` MS)))

(event `SetSlow`
  (params (MS :type "Float (double-precision)"))
  (if (`self.AllowCheat`)
    (`self.SetSlowEffect` MS)))

(event `SetRunningSpeed`
  (params (CurrentRunningSpeedMult :type "Float (double-precision)"))
  (if (`self.AllowCheat`)
    (set `self.CurrentRunningSpeedMult` CurrentRunningSpeedMult)))

(event `SetInventorySize`
  (params (MaxInventirySize :type Integer))
  (if (`self.AllowCheat`)
    (`/Game/_Mintbloom/Blueprints/Inventory/AC_Inventory.SetInventorySize` (`self.AC_Inventory`) MaxInventirySize)))

(fn `AddPoisoningBy`
  (params (Add :type "Float (double-precision)"))
  (returns (Return :type "Float (double-precision)"))
  (bind _output_get (set `self.PoisoningBar` (`KismetMathLibrary.FClamp` (+ (`self.PoisoningBar`) Add) 0.0 (`self.GetAttributeValueByTag` (struct :`TagName` "Attribute.Poison")))))
  (return _output_get))

(fn `AllowCheat`
  (returns (allow :type Boolean))
  (return (`self.CheatEnable`)))

(fn `ApplyEffect`
  (params (Effect :type "GameplayTag Structure") (Value :type "Float (double-precision)"))
  (`|SwitchGameplayTag` Effect
    (:`Effect.CurePoison`
      (`self.SetIsPoison` false))
    (:`Effect.IncreaseHungerBar`
      (`self.SetCurrentHunger` (+ (`self.GetCurrentHunger`) Value)))
    (:`Effect.Poison`
      (`self.SetIsPoison` true))
    (:`Effect.SlowMovementSpeed`
      (`self.SetSlowEffect` Value))))

(fn `ChangeStaminaBy`
  (params (Change :type "Float (double-precision)"))
  (returns (Output_Get :type "Float (double-precision)"))
  (bind _output_get (set `self.StaminaBar` (`KismetMathLibrary.FClamp` (+ (`self.StaminaBar`) Change) 0.0 (`self.GetAttributeValueByTag` (struct :`TagName` "Attribute.Stamina")))))
  (return _output_get))

(fn `CloseCurrentInteraction`
  (bind _returnvalue (`GameplayStatics.GetPlayerController` 0))
  (bind (_interaction _interactedwidgetonscreen) (`self.GetCurrentInteraction`))
  (`Widget.RemoveFromParent` _interactedwidgetonscreen)
  (`self.SetIsInteracting` false)
  ;[1 1 1] TBD
  (set `PlayerController.bShowMouseCursor` false _returnvalue)
  (`WidgetBlueprintLibrary.SetInputMode_GameOnly` _returnvalue))

(fn `FindEffectByItemID`
  (params (ItemId :type String))
  (returns (Effect :type "GameplayTag Structure") (Value :type "Float (double-precision)"))
  (locals (FoundIEffect :type Integer) (found :type Boolean :default false))
  (bind _outrownames (`DataTableFunctionLibrary.GetDataTableRowNames` "/Game/_Mintbloom/DT/ConsumableEffect.ConsumableEffect"))
  (for (_array_element _array_index) _outrownames
    (bind _returnvalue (`KismetStringLibrary.Contains` (`KismetStringLibrary.Conv_NameToString` _array_element) (`local.ItemId`)))
    (if _returnvalue
      (set `local.FoundIEffect` _array_index)
      (set `local.found` _returnvalue)
      (elif true
        _)))
  (if (`local.found`)
    (bind _returnvalue_2 (`|GetDataTableRow` "/Game/_Mintbloom/DT/ConsumableEffect.ConsumableEffect" (`|GetArrayItem` _outrownames (`local.FoundIEffect`)))
      (:`then`
        (bind (_itemtag _levels) (break `AttributeSystem` _returnvalue_2))
        (bind _keys (`BlueprintMapLibrary.Map_Keys` _levels))
        (bind _output (`|GetArrayItem` _keys))
        (return _output (`.Value` (break `LevelAttribute` (`.Level1` (break `LevelAttributeData` (`BlueprintMapLibrary.Map_Find` _levels _output)))))))
      (:`RowNotFound`
        _)))
  (return (struct) 0.0))

(fn `GetAttributeValueByTag`
  (params (Tag :type "GameplayTag Structure") (Level :type "/Game/_Mintbloom/Blueprints/Struct/AttributeLevel_E Enum" :default "NewEnumerator0"))
  (returns (Value :type "Float (double-precision)"))
  (bind (_level1 _level2 _level3 _level4 _level5) (break `LevelAttributeData` (`BlueprintMapLibrary.Map_Find` (`self.AttributeMap`) Tag)))
  (switch `/Game/_Mintbloom/Blueprints/Struct/AttributeLevel_E` Level
    (:`NewEnumerator0`
      (return (`.Value` (break `LevelAttribute` _level1))))
    (:`NewEnumerator1`
      (return (`.Value` (break `LevelAttribute` _level2))))
    (:`NewEnumerator2`
      (return (`.Value` (break `LevelAttribute` _level3))))
    (:`NewEnumerator3`
      (return (`.Value` (break `LevelAttribute` _level4))))
    (:`NewEnumerator4`
      (return (`.Value` (break `LevelAttribute` _level5))))))

(fn `GetCharacterCamera`
  (returns (Camera :type "CameraComponent Object Reference"))
  (return (`self.Camera`)))

(fn `GetCurrentHunger`
  (returns (Hunger :type "Float (double-precision)"))
  (return (`self.CurrentHunger`)))

(fn `GetCurrentInteraction`
  (returns (Interaction :type "GameplayTag Structure") (InteractedWidgetOnScreen :type "Widget Object Reference") (InteractedActor :type "Actor Object Reference"))
  (return (`self.CurrentIntection`) (`self.InteractedWidgetOnScreen`) (`self.Interacted Actor`)))

(fn `GetCurrentInteraction_I`
  (returns (InteractionType :type "GameplayTag Structure") (WidgetRef :type "Widget Object Reference") (InteractedActor :type "Actor Object Reference"))
  (bind (_interaction _interactedwidgetonscreen _interactedactor) (`self.GetCurrentInteraction`))
  (return _interaction _interactedwidgetonscreen _interactedactor))

(fn `GetCurrentWalkingSpeed`
  (returns (MS :type "Float (double-precision)"))
  (return (`self.CurrentMovementSpeed`)))

(fn `GetInventoryComponent`
  (returns (Conponent_ :type "/Game/_Mintbloom/Blueprints/Inventory/AC_Inventory Object Reference"))
  (return (`self.AC_Inventory`)))

(fn `GetIsInteract`
  (returns (IsInteract :type Boolean))
  (return (`self.IsInteract`)))

(fn `GetIsPoison`
  (returns (IsPoison :type Boolean))
  (return (`self.Is Poison`)))

(fn `GetIsRunning`
  (returns (IsRunning :type Boolean))
  (return (`self.Is Running`)))

(fn `GetSlowEffect`
  (returns (SlowEffectPercent :type "Float (double-precision)"))
  (return (`self.SlowEffectPercent`)))

(fn `GetUIHUD`
  (returns (Hud :type "/Game/_Mintbloom/Blueprints/UI/WBP_MainHUD Object Reference"))
  (bind _hud (message `/Game/_Mintbloom/Blueprints/Interface/HUDInteraction_I.GetMainHUD` (`PlayerController.GetHUD` (`GameplayStatics.GetPlayerController` 0))))
  (return _hud))

(fn `InitializeAttribute`
  (bind _valuepin (`|SetForEach` (`self.AttributeAbility`))
    (:`then`
      (`|SwitchGameplayTag` _valuepin
        (:`Attribute.MovementSpeed`
          (bind _output_get (set `CharacterMovementComponent.MaxWalkSpeed` (`self.GetAttributeValueByTag` (struct :`TagName` "Attribute.MovementSpeed")) (`self.CharacterMovement`)))
          (`self.SetCurrentWalkingSpeed` _output_get))
        (:`Attribute.Stamina`
          (set `self.StaminaBar` (`self.GetAttributeValueByTag` (struct :`TagName` "Attribute.Stamina"))))
        (:`Attribute.Hunger`
          (`self.SetCurrentHunger` 100.0))
        (:`Attribute.StaminaRecovery`
          (set `self.CurrentStaminaRecovery` (`self.GetAttributeValueByTag` (struct :`TagName` "Attribute.StaminaRecovery"))))
        (:`Attribute.HungerRate`
          (set `self.CurrentHungerRate` (`self.GetAttributeValueByTag` (struct :`TagName` "Attribute.HungerRate"))))
        (:`Attribute.RunningSpeed`
          (set `self.CurrentRunningSpeedMult` (`self.GetAttributeValueByTag` (struct :`TagName` "Attribute.RunningSpeed"))))))))

(fn `Interact`
  (params (InteractWith :type "Actor Object Reference"))
  (bind _interactwith (`local.InteractWith`))
  (bind _type (message `/Game/_Mintbloom/Blueprints/Interface/WorldInteraction_I.GetItemType` InteractWith))
  (`|SwitchGameplayTag` _type
    (:`ItemsType.CraftingStation`
      (`self.InteractCraftingStation`))
    (:`ItemsType.Interactable`
      (`self.InteractItem` _interactwith))
    (:`ItemsType.Pickable`
      (`self.PickUp` _interactwith))
    (:`ItemsType.Storage`
      (`self.InteractStorage` _interactwith)
      (`self.SetIsInteracting` true)
      (`self.ShowHideMouseCursor` true))))

(fn `InteractCraftingStation`)

(fn `InteractItem`
  (params (InteractWith :type "Actor Object Reference"))
  (message `/Game/_Mintbloom/Blueprints/Interface/WorldInteraction_I.Interact` InteractWith))

(fn `InteractStorage`
  (params (Chest :type "Actor Object Reference"))
  (bind _hud (`self.GetUIHUD`))
  (bind _isshowing (`/Game/_Mintbloom/Blueprints/UI/WBP_MainHUD.GetInventoryIsShowing` _hud))
  (if (not _isshowing)
    (`/Game/_Mintbloom/Blueprints/UI/WBP_MainHUD.ShowInventory` _hud true true))
  (bind _component (message `/Game/_Mintbloom/Blueprints/Interface/WorldInteraction_I.GetInventoryComponent` Chest))
  (bind _widgetonscreen (message `/Game/_Mintbloom/Blueprints/Interface/InventoryInteraction_I.AddOnScreen` _component true))
  (`self.SetCurrentInteraction` (struct :`TagName` "ItemsType.Storage") _widgetonscreen Chest))

(fn `PickUp`
  (params (InputPin :type "Object Object Reference"))
  ;[1 1 1] CheckForEmptySpace
  (if (> (`/Game/_Mintbloom/Blueprints/Inventory/AC_Inventory.GetInventoryEmptySlots` (`self.AC_Inventory`)) 0)
    (bind _nameid (message `/Game/_Mintbloom/Blueprints/Interface/ItemInteraction_I.GetItemNameID` InputPin))
    (`/Game/_Mintbloom/Blueprints/Inventory/AC_Inventory.AddItemToInventory` (`self.AC_Inventory`) _nameid)
    (message `/Game/_Mintbloom/Blueprints/Interface/ItemInteraction_I.PickedUp` InputPin)
    (bind _newparam (`/Game/_Mintbloom/Blueprints/UI/WBP_MainHUD.GetinventoryRef` (`self.GetUIHUD`)))
    (`/Game/_Mintbloom/Blueprints/UI/WBP_Inventory.AddItem` _newparam _nameid)))

(fn `RefreshUIStatBar`
  (params (NewValue :type "Float (double-precision)") (Param :type "/Game/_Mintbloom/Blueprints/Struct/UIStatBarAttribute_E Enum" :default "NewEnumerator0"))
  (returns (`%` :type "Float (double-precision)"))
  (bind _returnvalue (/ NewValue 100.0))
  (bind _returnvalue_2 (/ NewValue 100.0))
  (bind _returnvalue_3 (/ NewValue (`self.GetAttributeValueByTag` (struct :`TagName` "Attribute.Stamina"))))
  (switch `/Game/_Mintbloom/Blueprints/Struct/UIStatBarAttribute_E` Param
    (:`NewEnumerator0`
      (`/Game/_Mintbloom/Blueprints/UI/WBP_MainHUD.SetStaminaBar` (`self.GetUIHUD`) _returnvalue_3)
      (return _returnvalue_3))
    (:`NewEnumerator1`
      (`/Game/_Mintbloom/Blueprints/UI/WBP_MainHUD.SetHungerBar` (`self.GetUIHUD`) _returnvalue_2)
      (return _returnvalue_2))
    (:`NewEnumerator2`
      (`/Game/_Mintbloom/Blueprints/UI/WBP_MainHUD.SetPoisonBar` (`self.GetUIHUD`) _returnvalue)
      (return _returnvalue))))

(fn `SetCurrentHunger`
  (params (Hunger :type "Float (double-precision)"))
  (set `self.CurrentHunger` (`KismetMathLibrary.FClamp` Hunger 0.0 100.0))
  (return))

(fn `SetCurrentInteraction`
  (params (Interaction :type "GameplayTag Structure") (WidgetOnScreen :type "Widget Object Reference") (InteractedActor :type "Actor Object Reference"))
  (set `self.CurrentIntection` Interaction)
  (set `self.InteractedWidgetOnScreen` WidgetOnScreen)
  (set `self.Interacted Actor` InteractedActor))

(fn `SetCurrentWalkingSpeed`
  (params (MS :type "Float (double-precision)"))
  (set `self.CurrentMovementSpeed` MS)
  (return))

(fn `SetIsInteracting`
  (params (SetIsInteracting :type Boolean))
  (set `self.IsInteract` SetIsInteracting)
  (return))

(fn `SetIsPoison`
  (params (IsPoison :type Boolean))
  (set `self.Is Poison` IsPoison))

(fn `SetIsRunning`
  (params (IsRunning :type Boolean))
  (set `self.Is Running` IsRunning))

(fn `SetSlowEffect`
  (params (SlowEffectPercent :type "Float (double-precision)"))
  (if (> SlowEffectPercent (`self.GetSlowEffect`))
    (set `self.SlowEffectPercent` SlowEffectPercent)))

(fn `ShowHideInventory`
  (returns (Currently :type Boolean))
  (bind _hud (`self.GetUIHUD`))
  (bind _isshowing (`/Game/_Mintbloom/Blueprints/UI/WBP_MainHUD.GetInventoryIsShowing` _hud))
  (`/Game/_Mintbloom/Blueprints/UI/WBP_MainHUD.ShowInventory` _hud (not _isshowing) false)
  (bind _isshowing_2 (`/Game/_Mintbloom/Blueprints/UI/WBP_MainHUD.GetInventoryIsShowing` (`self.GetUIHUD`)))
  (return _isshowing_2))

(fn `ShowHideMouseCursor`
  (params (SetIsShow :type Boolean))
  (bind _output_get (set `PlayerController.bShowMouseCursor` SetIsShow (`GameplayStatics.GetPlayerController` 0)))
  (if _output_get
    (`WidgetBlueprintLibrary.SetInputMode_GameAndUIEx` (`GameplayStatics.GetPlayerController` 0) (`self.GetUIHUD`))
    (else
      (`WidgetBlueprintLibrary.SetInputMode_GameOnly` (`GameplayStatics.GetPlayerController` 0)))))

(fn `UserConstructionScript`
  (bind _returnvalue (`|GetDataTableRow` (`self.Characted_DT`) (`BlueprintGameplayTagLibrary.GetTagName` (`BlueprintGameplayTagLibrary.MakeLiteralGameplayTag` (struct :`TagName` "Player"))))
    (:`then`
      (set `self.AttributeMap` (`.Levels` (break `AttributeSystem` _returnvalue)))
      (`self.InitializeAttribute`))))