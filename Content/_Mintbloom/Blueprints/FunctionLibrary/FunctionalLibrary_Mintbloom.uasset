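; Blueprint function library for Mintbloom that resolves brew and food item IDs into effect data from the ConsumableEffect table.
; GetBrewInfo peels up to three underscore-separated ingredients off a Brew ID, using AddMapWithEffect to read each one's first-key effect and duration at Level1.
; A repeated effect overwrites its entry with value and duration doubled or tripled by ingredient position.
; GetFoodInfo returns Level1 nutrient values; FindBuildActor is empty.
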(fn `AddMapWithEffect`
  (params (RowName :type Name))
  (returns (Effect :type "GameplayTag Structure (by ref)") (Value :type "Float (single-precision)") (Duration :type "Float (double-precision)"))
  (bind _returnvalue (`|GetDataTableRow` "/Game/_Mintbloom/DT/ConsumableEffect.ConsumableEffect" RowName)
    (:`then`
      (bind (_itemtag _levels) (break `AttributeSystem` _returnvalue))
      (bind _keys (`BlueprintMapLibrary.Map_Keys` _levels))
      (bind _output (`|GetArrayItem` _keys))
      (return _output (`.Value` (break `LevelAttribute` (`.Level1` (break `LevelAttributeData` (`BlueprintMapLibrary.Map_Find` _levels _output))))) (`.Value` (break `LevelAttribute` (`.Level1` (break `LevelAttributeData` (`BlueprintMapLibrary.Map_Find` _levels (struct :`TagName` "Attribute.Duration"))))))))
    (:`RowNotFound`
      (return (struct) 0.0 0.0))))

(fn `FindBuildActor`)

(fn `GetBrewInfo`
  (params (ItemID :type String))
  (returns (Effect :type "Map of GameplayTag Structure to /Game/_Mintbloom/DT/Effect_s Structure"))
  (locals (ReturnMap :type "Map of GameplayTag Structure to /Game/_Mintbloom/DT/Effect_s Structure"))
  (bind (_lefts _rights) (`KismetStringLibrary.Split` ItemID "_" "IgnoreCase" "FromEnd"))
  (bind (_lefts_2 _rights_2) (`KismetStringLibrary.Split` _lefts "_" "IgnoreCase" "FromEnd"))
  (bind (_effect _value _duration) (`self.AddMapWithEffect` (`KismetStringLibrary.Conv_StringToName` _rights)))
  (`BlueprintMapLibrary.Map_Add` (`local.ReturnMap`) _effect (make `/Game/_Mintbloom/DT/Effect_s` _value _duration))
  (if (`KismetStringLibrary.EqualEqual_StrStr` _lefts "Brew")
    (return (`local.ReturnMap`))
    (else
      (bind (_effect_2 _value_2 _duration_2) (`self.AddMapWithEffect` (`KismetStringLibrary.Conv_StringToName` _rights_2)))
      (if (`BlueprintMapLibrary.Map_Contains` (`local.ReturnMap`) _effect_2)
        (`BlueprintMapLibrary.Map_Add` (`local.ReturnMap`) _effect_2 (make `/Game/_Mintbloom/DT/Effect_s` (* _value_2 2.0) (* _duration_2 2.0)))
        (else
          (`BlueprintMapLibrary.Map_Add` (`local.ReturnMap`) _effect_2 (make `/Game/_Mintbloom/DT/Effect_s` _value_2 _duration_2))))
      (if (`KismetStringLibrary.EqualEqual_StrStr` _lefts_2 "Brew")
        (return (`local.ReturnMap`))
        (else
          (bind (_effect_3 _value_3 _duration_3) (`self.AddMapWithEffect` (`KismetStringLibrary.Conv_StringToName` (`.RightS` (`KismetStringLibrary.Split` _lefts_2 "_" "IgnoreCase" "FromEnd")))))
          (if (`BlueprintMapLibrary.Map_Contains` (`local.ReturnMap`) _effect_3)
            (`BlueprintMapLibrary.Map_Add` (`local.ReturnMap`) _effect_3 (make `/Game/_Mintbloom/DT/Effect_s` (* _value_3 3.0) (* _duration_3 3.0)))
            (return (`local.ReturnMap`))
            (else
              (`BlueprintMapLibrary.Map_Add` (`local.ReturnMap`) _effect_3 (make `/Game/_Mintbloom/DT/Effect_s` _value_3 _duration_3))
              (return (`local.ReturnMap`)))))))))

(fn `GetFoodInfo`
  (params (NameID :type String))
  (returns (FoodQuality :type "/Game/_Mintbloom/DT/Food_s Structure"))
  (bind _returnvalue (`|GetDataTableRow` "/Game/_Mintbloom/DT/ConsumableEffect.ConsumableEffect" (`KismetStringLibrary.Conv_StringToName` NameID))
    (:`then`
      (bind (_itemtag _levels) (break `AttributeSystem` _returnvalue))
      (return (make `/Game/_Mintbloom/DT/Food_s` (`.Value` (break `LevelAttribute` (`.Level1` (break `LevelAttributeData` (`BlueprintMapLibrary.Map_Find` _levels (struct :`TagName` "Food.Proteins")))))) (`.Value` (break `LevelAttribute` (`.Level1` (break `LevelAttributeData` (`BlueprintMapLibrary.Map_Find` _levels (struct :`TagName` "Food.Fats")))))) (`.Value` (break `LevelAttribute` (`.Level1` (break `LevelAttributeData` (`BlueprintMapLibrary.Map_Find` _levels (struct :`TagName` "Food.Carbs")))))) (`.Value` (break `LevelAttribute` (`.Level1` (break `LevelAttributeData` (`BlueprintMapLibrary.Map_Find` _levels (struct :`TagName` "Food.DietFiber")))))))))
    (:`RowNotFound`
      (return))))