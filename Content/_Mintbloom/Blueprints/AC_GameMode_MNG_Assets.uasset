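; Game mode asset manager component that builds a runtime list of the game's items and provides lookup by name.
; On BeginPlay it queries the Asset Registry for PDA_Item data assets, excluding subclasses, and flattens their Item arrays into one Items list.
; FItemFindByName linearly searches that list, returning the matching item and a validity flag.
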(event `self.ReceiveBeginPlay`
  (`|ExecutionSequence`
    (:`then_0`
      ;[1 1 1] Load Items
      (bind _outassetdata (`AssetRegistry.GetAssetsByClass` (`AssetRegistryHelpers.GetAssetRegistry`) (`KismetSystemLibrary.GetClassTopLevelAssetPath` "/Game/_Mintbloom/PDA/PDA_Item.PDA_Item_C") false))
      (for _array_element _outassetdata
        (bind _aspda_item (cast `/Game/_Mintbloom/PDA/PDA_Item` (`AssetRegistryHelpers.GetAsset` _array_element)))
        (for _array_element_2 (`/Game/_Mintbloom/PDA/PDA_Item.Item` _aspda_item)
          (`KismetArrayLibrary.Array_Add` (`self.Items`) _array_element_2))))))

(fn `F_Item_Find_ByName`
  (params (Name :type String))
  (returns (Item :type "/Game/_Mintbloom/Blueprints/Inventory/STR_Item Structure") (Valid :type Boolean))
  ;[1 1 1] Comment
  (for _array_element (`self.Items`)
    (if (== Name (`KismetTextLibrary.Conv_TextToString` (`.Name_3_888C6473449A50127FEBC6B0306D6862` (break `/Game/_Mintbloom/Blueprints/Inventory/STR_Item` _array_element))))
      (return _array_element true)))
  ;[1 1 1] Comment
  (return (struct) false))